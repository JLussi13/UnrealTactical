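; BP_Grid lays out a flat grid of shaped tiles, rebuilt from the Construction Script.
; SpawnGrid stores its layout inputs and looks up the shape's row in DT_GridShapeData to set the InstancedStaticMesh's flat mesh and border material.
; A nested X/Y loop adds local-space instances at zero Z, spaced by GridSize and offset by half the grid extent from Center.
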(fn `SpawnGrid`
  (params (Center :type "Vector Structure") (GridSize :type "Vector Structure") (TileCount :type "Vector2D Structure") (Shape :type "/Game/Blueprints/Core/Grid/GridShapes/E_GridShape Enum" :default "NewEnumerator3"))
  (locals (CurrentShapeData :type "/Game/Blueprints/Core/Grid/GridShapes/S_GridShapeData Structure") (StartSpawn :type "Vector Structure"))
  (bind _instancedstaticmesh (`self.InstancedStaticMesh`))
  (bind (_grid_size_x _grid_size_y) (`KismetMathLibrary.BreakVector` (`self.Grid Size`)))
  (bind _grid_size_x_2 (`KismetMathLibrary.BreakVector` (`self.Grid Size`)))
  (bind (_startspawn_x _startspawn_y) (`KismetMathLibrary.BreakVector` (`local.StartSpawn`)))
  (bind _startspawn_x_2 (`KismetMathLibrary.BreakVector` (`local.StartSpawn`)))
  (bind (_tile_count_x _tile_count_y) (`KismetMathLibrary.BreakVector2D` (`self.Tile Count`)))
  (set `self.Center` Center)
  (set `self.Grid Size` GridSize)
  (set `self.Tile Count` TileCount)
  (set `self.Shape` Shape)
  (bind _returnvalue (`|GetDataTableRow` "/Game/Blueprints/Core/Grid/GridShapes/DT_GridShapeData.DT_GridShapeData" (`KismetStringLibrary.Conv_StringToName` (`|GetEnumeratorNameAsString` (`self.Shape`))))
    (:`then`
      (set `local.CurrentShapeData` _returnvalue)
      (bind (_meshsize _mesh _meshmaterial _flatmesh _flatbordermaterial) (break `/Game/Blueprints/Core/Grid/GridShapes/S_GridShapeData` _returnvalue))
      (`StaticMeshComponent.SetStaticMesh` _instancedstaticmesh _flatmesh)
      (`PrimitiveComponent.SetMaterial` _instancedstaticmesh 0 _flatbordermaterial)
      (set `local.StartSpawn` (- (`self.Center`) (/ (* (`self.Grid Size`) (`self.Tile Count`)) (2.0 2.0 2.0))))
      (for _index (range (+ (`KismetMathLibrary.FTrunc` _tile_count_x) 1))
        (for _index_2 (range (+ (`KismetMathLibrary.FTrunc` _tile_count_y) 1))
          (`InstancedStaticMeshComponent.AddInstance` (`self.InstancedStaticMesh`) (`KismetMathLibrary.Conv_VectorToTransform` (`KismetMathLibrary.MakeVector` (+ (* _index _grid_size_x_2) _startspawn_x_2) (+ (* _index_2 _grid_size_y) _startspawn_y))) false))))))

(fn `UserConstructionScript`
  (`self.SpawnGrid` (`self.Center`) (`self.Grid Size`) (`self.Tile Count`) (`self.Shape`)))