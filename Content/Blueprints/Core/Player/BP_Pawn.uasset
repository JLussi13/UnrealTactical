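; BP_Pawn is a player camera pawn with spring-arm zoom, planar movement and stepped rotation.
; Input axes adjust a clamped zoom target and move the location target along the actor's forward and right vectors, while action presses rotate the rotation target in 45-degree steps.
; Tick eases arm length, location and rotation toward those targets with interpolation at a shared speed, giving smoothed motion without collision sweeps.
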(event `self.ReceiveBeginPlay`
  (set `self.ZoomLerped` (`SpringArmComponent.TargetArmLength` (`self.SpringArm`)))
  (set `self.LocationLerped` (`self.K2_GetActorLocation`))
  (set `self.RotationLerped` (`self.K2_GetActorRotation`)))

(event `self.ReceiveTick`
  (params (DeltaSeconds :type "Float (single-precision)"))
  (set `SpringArmComponent.TargetArmLength` (`KismetMathLibrary.FInterpTo` (`SpringArmComponent.TargetArmLength` (`self.SpringArm`)) (`self.ZoomLerped`) (`GameplayStatics.GetWorldDeltaSeconds`) (`self.Interp Speed`)) (`self.SpringArm`))
  (`self.K2_SetActorLocation` (`KismetMathLibrary.VInterpTo` (`self.K2_GetActorLocation`) (`self.LocationLerped`) (`GameplayStatics.GetWorldDeltaSeconds`) (`self.Interp Speed`)))
  (`self.K2_SetActorRotation` (`KismetMathLibrary.RInterpTo` (`self.K2_GetActorRotation`) (`self.RotationLerped`) (`GameplayStatics.GetWorldDeltaSeconds`) (`self.Interp Speed`))))

(event `InputAxis|InputAxisZoom`
  (params (AxisValue :type "Float (single-precision)"))
  (set `self.ZoomLerped` (`KismetMathLibrary.FClamp` (+ (`self.ZoomLerped`) (* AxisValue (`self.ZoomSpeed`))) 100.0 5000.0)))

(event `InputAxis|InputAxisForward`
  (params (AxisValue :type "Float (single-precision)"))
  (set `self.LocationLerped` (+ (`self.LocationLerped`) (* (* AxisValue (`self.MoveSpeed`)) (`self.GetActorForwardVector`)))))

(event `InputAxis|InputAxisRight`
  (params (AxisValue :type "Float (single-precision)"))
  (set `self.LocationLerped` (+ (`self.LocationLerped`) (* (* AxisValue (`self.MoveSpeed`)) (`self.GetActorRightVector`)))))

(event `InputAction|InputActionRotationRight`
  (params (Key :type "Key Structure"))
  (:`Pressed`
    (set `self.RotationLerped` (`KismetMathLibrary.ComposeRotators` (`self.RotationLerped`) (struct :`Yaw` -45.0)))))

(event `InputAction|InputActionRotationLeft`
  (params (Key :type "Key Structure"))
  (:`Pressed`
    (set `self.RotationLerped` (`KismetMathLibrary.ComposeRotators` (`self.RotationLerped`) (struct :`Yaw` 45.0)))))

(fn `UserConstructionScript`)